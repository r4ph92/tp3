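; Player state for a maze game that holds the victory check based on collected coins and opened chests.
; CheckVictory compares both counters against hardcoded minimums and, when both are met, casts the game mode to BP_MazeGameMode and ends the game as a win.
; The event graph is empty, so the counters are not updated and the check is not triggered within this Blueprint.
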(fn `CheckVictory`
  (if (and (>= (`self.CoinsCollected`) 10) (>= (`self.ChestsOpened`) 1))
    (bind _asbp_maze_game_mode (cast `/Game/Blueprints/BP_MazeGameMode` (`GameplayStatics.GetGameMode`)))
    (`/Game/Blueprints/BP_MazeGameMode.EndGame` _asbp_maze_game_mode true)))

(fn `UserConstructionScript`)