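; Game mode for the maze game that handles the end of a match as a win or a loss.
; EndGame runs only once via a GameEnded flag and creates either the victory or game-over widget depending on the Victory input.
; It then switches player 0 to UI-only input focused on that widget, shows the mouse cursor and pauses the game.
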(fn `EndGame`
  (params (bVictory :type Boolean))
  (bind _returnvalue (`GameplayStatics.GetPlayerController` 0))
  (if (not (`self.bGameEnded`))
    (set `self.bGameEnded` true)
    (if bVictory
      (bind _returnvalue_2 (`|CreateWidget` "/Game/Blueprints/WBP_Victory.WBP_Victory_C" _returnvalue))
      (`UserWidget.AddToViewport` _returnvalue_2 0)
      (`WidgetBlueprintLibrary.SetInputMode_UIOnlyEx` _returnvalue _returnvalue_2)
      (else
        (bind _returnvalue_3 (`|CreateWidget` "/Game/Blueprints/WBP_GameOver.WBP_GameOver_C" _returnvalue))
        (`UserWidget.AddToViewport` _returnvalue_3 0)
        (`WidgetBlueprintLibrary.SetInputMode_UIOnlyEx` _returnvalue _returnvalue_3)))
    (set `PlayerController.bShowMouseCursor` true _returnvalue)
    (`GameplayStatics.SetGamePaused` true)))

(fn `UserConstructionScript`)