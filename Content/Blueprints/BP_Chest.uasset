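; BP_Chest is an openable maze chest that counts toward the player's victory condition.
; Its interaction sphere sets or clears itself as the character's CurrentChest on overlap and prints a key prompt.
; OpenChest works only once: it starts a timeline that rotates the lid pivot, increments ChestsOpened on BP_MazePlayerState, checks victory and refreshes the character's HUD.
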(event `self.InteractionSphere.OnComponentBeginOverlap`
  (params (OverlappedComponent :type "PrimitiveComponent Object Reference") (OtherActor :type "Actor Object Reference") (OtherComp :type "PrimitiveComponent Object Reference") (OtherBodyIndex :type Integer) (bFromSweep :type Boolean) (SweepResult :type "HitResult Structure (by ref)"))
  (bind _asbp_third_person_character (cast `/Game/ThirdPerson/Blueprints/BP_ThirdPersonCharacter` OtherActor))
  (set `self.PlayerInRange` true)
  (set `/Game/ThirdPerson/Blueprints/BP_ThirdPersonCharacter.CurrentChest` self _asbp_third_person_character)
  (`KismetSystemLibrary.PrintString` "press E to open chest"))

(event `AnimateChestOpening`
  (bind (_direction _openalpha) (`Timeline|TL_ChestOpening` :!via `PlayFromStart`)
    (:`Update`
      (`SceneComponent.K2_SetRelativeRotation` (`self.LidPivot`) (`KismetMathLibrary.RLerp` (struct) (struct :`Roll` 90.0) _openalpha) false false))))

(event `self.InteractionSphere.OnComponentEndOverlap`
  (params (OverlappedComponent :type "PrimitiveComponent Object Reference") (OtherActor :type "Actor Object Reference") (OtherComp :type "PrimitiveComponent Object Reference") (OtherBodyIndex :type Integer))
  (bind _asbp_third_person_character (cast `/Game/ThirdPerson/Blueprints/BP_ThirdPersonCharacter` OtherActor))
  (set `self.PlayerInRange` false)
  (set `/Game/ThirdPerson/Blueprints/BP_ThirdPersonCharacter.CurrentChest` null _asbp_third_person_character))

(fn `OpenChest`
  (if (not (`self.IsOpened`))
    (set `self.IsOpened` true)
    (`self.AnimateChestOpening`)
    (bind _asbp_maze_player_state (cast `/Game/Blueprints/BP_MazePlayerState` (`GameplayStatics.GetPlayerState` 0)))
    (bind _output_get (set `/Game/Blueprints/BP_MazePlayerState.ChestsOpened` (+ (`/Game/Blueprints/BP_MazePlayerState.ChestsOpened` _asbp_maze_player_state) 1) _asbp_maze_player_state))
    (`/Game/Blueprints/BP_MazePlayerState.CheckVictory` _asbp_maze_player_state)
    (bind _asbp_third_person_character (cast `/Game/ThirdPerson/Blueprints/BP_ThirdPersonCharacter` (`GameplayStatics.GetPlayerCharacter` 0)))
    (`/Game/Blueprints/WBP_HUD.UpdateHUD` (`/Game/ThirdPerson/Blueprints/BP_ThirdPersonCharacter.HUDReference` _asbp_third_person_character))
    (`KismetSystemLibrary.PrintString` "Chest opened!")
    (`KismetSystemLibrary.PrintString` (`KismetStringLibrary.Conv_IntToString` _output_get))))

(fn `UserConstructionScript`)