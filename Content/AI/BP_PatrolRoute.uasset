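; BP_PatrolRoute is a placeable actor that defines a patrol route for AI, using the child components of its root as the patrol points.
; GetPatrolPoint returns a child's world location, wrapping the index by the child count, or the actor's own location when there are no children.
; GetPatrolPointCount reports the number of direct children, and the event graph holds no active logic.
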(fn `GetPatrolPoint`
  (params (Index :type Integer))
  (returns (Location :type "Vector Structure"))
  (bind _children (`SceneComponent.GetChildrenComponents` (`self.RootComponent`) false))
  (bind _returnvalue (`KismetArrayLibrary.Array_Length` _children))
  (if (> _returnvalue 0)
    (return (`SceneComponent.K2_GetComponentLocation` (`|GetArrayItem` _children (mod Index _returnvalue))))
    (else
      (return (`self.K2_GetActorLocation`)))))

(fn `GetPatrolPointCount`
  (returns (Count :type Integer))
  (return (`KismetArrayLibrary.Array_Length` (`SceneComponent.GetChildrenComponents` (`self.RootComponent`) false))))

(fn `UserConstructionScript`)