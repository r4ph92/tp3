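; BP_NPC is a maze-game guard character that ends the game as a loss when the player pawn overlaps its CatchZone.
; SetGuardState switches between passive, alert and chasing, updating the French state label, its color and the walk speed, which rises with each state.
; The guard starts passive, and this Blueprint contains no logic that triggers the other states.
; Every tick, the state text rotates to face the player camera.
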(event `self.ReceiveBeginPlay`
  (`self.SetGuardState` 0))

(event `self.CatchZone.OnComponentBeginOverlap`
  (params (OverlappedComponent :type "PrimitiveComponent Object Reference") (OtherActor :type "Actor Object Reference") (OtherComp :type "PrimitiveComponent Object Reference") (OtherBodyIndex :type Integer) (bFromSweep :type Boolean) (SweepResult :type "HitResult Structure (by ref)"))
  (if (== OtherActor (`GameplayStatics.GetPlayerPawn` 0))
    (bind _asbp_maze_game_mode (cast `/Game/Blueprints/BP_MazeGameMode` (`GameplayStatics.GetGameMode`)))
    (`/Game/Blueprints/BP_MazeGameMode.EndGame` _asbp_maze_game_mode false)))

(event `self.ReceiveTick`
  (params (DeltaSeconds :type "Float (single-precision)"))
  (bind _statetext (`self.StateText`))
  (`SceneComponent.K2_SetWorldRotation` _statetext (`KismetMathLibrary.FindLookAtRotation` (`SceneComponent.K2_GetComponentLocation` _statetext) (`PlayerCameraManager.GetCameraLocation` (`GameplayStatics.GetPlayerCameraManager` 0))) false false))

(fn `SetGuardState`
  (params (State :type Integer))
  (bind _charactermovement (`self.CharacterMovement`))
  (switch `int` State
    (:`0`
      (`TextRenderComponent.K2_SetText` (`self.StateText`) (`KismetTextLibrary.Conv_StringToText` "Passif"))
      (`TextRenderComponent.SetTextRenderColor` (`self.StateText`) (struct :`B` 80 :`G` 255 :`R` 80 :`A` 255))
      (set `CharacterMovementComponent.MaxWalkSpeed` 200.0 _charactermovement))
    (:`1`
      (`TextRenderComponent.K2_SetText` (`self.StateText`) (`KismetTextLibrary.Conv_StringToText` "Alerte"))
      (`TextRenderComponent.SetTextRenderColor` (`self.StateText`) (struct :`G` 200 :`R` 255 :`A` 255))
      (set `CharacterMovementComponent.MaxWalkSpeed` 300.0 _charactermovement))
    (:`2`
      (`TextRenderComponent.K2_SetText` (`self.StateText`) (`KismetTextLibrary.Conv_StringToText` "En chasse"))
      (`TextRenderComponent.SetTextRenderColor` (`self.StateText`) (struct :`B` 40 :`G` 40 :`R` 255 :`A` 255))
      (set `CharacterMovementComponent.MaxWalkSpeed` 450.0 _charactermovement))))

(fn `UserConstructionScript`)