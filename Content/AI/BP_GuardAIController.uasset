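; AI controller for guard NPCs that patrol and react to seeing or losing the player.
; On possess it runs the guard behavior tree, and perception updates write the player as blackboard target, or the last stimulus location when sensing is lost.
; GetNextPatrolLocation steps through the BP_NPC's patrol route with a wrapping index, falling back to the pawn's own location without a valid route.
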(event `self.ReceivePossess`
  (params (PossessedPawn :type "Pawn Object Reference"))
  (`self.RunBehaviorTree` self (`self.GuardBehaviorTree`)))

(event `self.AIPerception.OnTargetPerceptionUpdated`
  (params (Actor :type "Actor Object Reference") (Stimulus :type "AIStimulus Structure"))
  (bind (_age _expirationage _strength _stimuluslocation _receiverlocation _tag _bsuccessfullysensed) (break `AIStimulus` Stimulus))
  (bind _returnvalue (`AIBlueprintHelperLibrary.GetBlackboard` self))
  (if (== Actor (`GameplayStatics.GetPlayerPawn` 0))
    (if _bsuccessfullysensed
      (`BlackboardComponent.SetValueAsObject` _returnvalue (`self.TargetKeyName`) Actor)
      (`BlackboardComponent.ClearValue` _returnvalue (`self.LastKnownLocationKeyName`))
      (else
        (`BlackboardComponent.ClearValue` _returnvalue (`self.TargetKeyName`))
        (`BlackboardComponent.SetValueAsVector` _returnvalue (`self.LastKnownLocationKeyName`) _stimuluslocation)))))

(fn `GetNextPatrolLocation`
  (returns (Location :type "Vector Structure"))
  (bind _asbp_npc (cast `/Game/AI/NPC/BP_NPC` (`self.K2_GetPawn`))
    (:`then`
      (bind _patrolroute (`/Game/AI/NPC/BP_NPC.PatrolRoute` _asbp_npc))
      (`/Engine/EditorBlueprintResources/StandardMacros.IsValid` _patrolroute
        (:`Is Valid`
          (bind _location (`/Game/AI/BP_PatrolRoute.GetPatrolPoint` _patrolroute (`self.PatrolIndex`)))
          (bind _count (`/Game/AI/BP_PatrolRoute.GetPatrolPointCount` _patrolroute))
          (set `self.PatrolIndex` (mod (+ (`self.PatrolIndex`) 1) (select `bool` (> _count 0) :`false` 1 :`true` _count)))
          (return _location))
        (:`Is Not Valid`
          (return (`self.K2_GetActorLocation` _asbp_npc)))))
    (:`CastFailed`
      (return (`self.K2_GetActorLocation`)))))

(fn `UserConstructionScript`)